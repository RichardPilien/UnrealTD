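; BP_Enemy5 is an enemy actor that travels along a level path and destroys itself when it reaches the end.
; On BeginPlay it finds a BP_Path actor with GetActorOfClass and, after a short delay, starts a Timeline.
; The Timeline's alpha is lerped over the spline length to set the actor's world location and rotation, so the Timeline sets the travel time regardless of path length.
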(event `self.ReceiveBeginPlay`
  ;[1 1 1] Getting Actor Reference and Calling Custom Event
  (bind _returnvalue (`GameplayStatics.GetActorOfClass` "/Game/Blueprints/BP_Path/BP_Path.BP_Path_C"))
  (set `self.Path` _returnvalue)
  (`self.Start Moving`))

(event `Start Moving`
  ;[1 1 1] Doing The Event Calling Path Reference and getting Length of the spline + setting actor and location of the spline
  (`KismetSystemLibrary.Delay` 1.0)
  (bind (_direction _alpha) (`Timeline|Timeline`)
    (:`Update`
      (bind (_returnvalue_location _returnvalue_rotation) (`KismetMathLibrary.BreakTransform` (`SplineComponent.GetTransformAtDistanceAlongSpline` (`/Game/Blueprints/BP_Path/BP_Path.Spline` (`self.Path`)) (`KismetMathLibrary.Lerp` 0.0 (`SplineComponent.GetSplineLength` (`/Game/Blueprints/BP_Path/BP_Path.Spline` (`self.Path`))) _alpha) "World" false)))
      (`self.K2_SetActorLocationAndRotation` _returnvalue_location _returnvalue_rotation))
    (:`Finished`
      (`self.K2_DestroyActor`))))

(fn `UserConstructionScript`)