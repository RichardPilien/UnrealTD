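; BP_Enemy7 is an enemy actor that travels along the spline of a BP_Path2 actor found in the level at BeginPlay.
; Each tick it advances a distance by Speed and sets its transform from that spline point, using the mesh's relative scale.
; When IsLooping is set, the distance resets to zero past the spline's end.
; Mesh overlaps with a BP_Projectile only store a reference to it.
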(event `self.ReceiveBeginPlay`
  (bind _returnvalue (`GameplayStatics.GetActorOfClass` "/Game/Blueprints/BP_Path/BP_Path2.BP_Path2_C"))
  (set `self.Path2` _returnvalue))

(event `self.Mesh.OnComponentBeginOverlap`
  (params (OverlappedComponent :type "PrimitiveComponent Object Reference") (OtherActor :type "Actor Object Reference") (OtherComp :type "PrimitiveComponent Object Reference") (OtherBodyIndex :type Integer) (bFromSweep :type Boolean) (SweepResult :type "HitResult Structure (by ref)"))
  (bind _asbp_projectile (cast `/Game/Blueprints/BP_Units/BP_Projectile` OtherActor))
  (set `self.As BP Projectile` _asbp_projectile))

(event `self.ReceiveTick`
  (params (DeltaSeconds :type "Float (single-precision)"))
  (bind (_returnvalue_location _returnvalue_rotation) (`KismetMathLibrary.BreakTransform` (`SplineComponent.GetTransformAtDistanceAlongSpline` (`/Game/Blueprints/BP_Path/BP_Path2.ESpline` (`self.Path2`)) (`self.Distance`) "World" false)))
  (set `self.Distance` (+ (* DeltaSeconds (`self.Speed`)) (`self.Distance`)))
  (`self.K2_SetActorTransform` (`KismetMathLibrary.MakeTransform` _returnvalue_location _returnvalue_rotation (`SceneComponent.RelativeScale3D` (`self.Mesh`))))
  (if (`self.isLooping?`)
    (if (> (`self.Distance`) (`SplineComponent.GetSplineLength` (`/Game/Blueprints/BP_Path/BP_Path2.ESpline` (`self.Path2`))))
      (set `self.Distance` 0.0))))

(fn `UserConstructionScript`)