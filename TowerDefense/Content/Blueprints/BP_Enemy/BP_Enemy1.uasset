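; BP_Enemy1 is an enemy Blueprint that moves its mesh along a spline path.
; Each tick it adds Speed times delta time to an accumulated distance, then samples the spline's local-space transform at that distance.
; It applies that location and rotation to the mesh's relative transform while keeping the mesh's own scale.
; The distance is never reset or wrapped.
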(event `self.ReceiveTick`
  (params (DeltaSeconds :type "Float (single-precision)"))
  (bind _mesh (`self.Mesh`))
  (bind (_returnvalue_location _returnvalue_rotation) (`KismetMathLibrary.BreakTransform` (`SplineComponent.GetTransformAtDistanceAlongSpline` (`self.Spline`) (`self.DistanceAll`) "Local" false)))
  (set `self.DistanceAll` (+ (* DeltaSeconds (`self.Speed`)) (`self.DistanceAll`)))
  (`SceneComponent.K2_SetRelativeTransform` _mesh (`KismetMathLibrary.MakeTransform` _returnvalue_location _returnvalue_rotation (`SceneComponent.RelativeScale3D` _mesh)) false false))

(fn `UserConstructionScript`)