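; BP_Enemy2 is an enemy Blueprint that moves its Enemy2 component along a spline path.
; Each Tick advances the travelled distance by SplineSpeed times delta time, then applies the spline's local-space location and rotation as the component's relative transform, preserving its scale.
; The distance is never wrapped, clamped or reversed, so the Blueprint itself has no looping or end-of-path handling.
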(event `self.ReceiveTick`
  (params (DeltaSeconds :type "Float (single-precision)"))
  (bind _enemy2 (`self.Enemy2`))
  (bind (_returnvalue_location _returnvalue_rotation) (`KismetMathLibrary.BreakTransform` (`SplineComponent.GetTransformAtDistanceAlongSpline` (`self.Spline`) (`self.Distance_along_spine`) "Local" false)))
  (set `self.Distance_along_spine` (+ (* DeltaSeconds (`self.Spline_Speed`)) (`self.Distance_along_spine`)))
  (`SceneComponent.K2_SetRelativeTransform` _enemy2 (`KismetMathLibrary.MakeTransform` _returnvalue_location _returnvalue_rotation (`SceneComponent.RelativeScale3D` _enemy2)) false false))

(fn `UserConstructionScript`)