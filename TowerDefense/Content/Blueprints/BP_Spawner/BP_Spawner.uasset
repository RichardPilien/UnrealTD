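; BP_Spawner is a spawner that keeps placing BP_Enemy2 enemies on the world's static geometry.
; A looping timer started on BeginPlay fires the spawn event every couple of seconds.
; Each tick traces from high above its location along the negative actor up vector against WorldStatic objects, then spawns an enemy at the impact point without checking for a hit.
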(event `self.ReceiveBeginPlay`
  (`KismetSystemLibrary.K2_SetTimerDelegate` (delegate `SpawningLoop_event`) 2.0 true))

(event `SpawningLoop_event`
  (bind _returnvalue (`KismetMathLibrary.MakeVector` (.x (`self.Location`)) (.y (`self.Location`)) (+ (.z (`self.Location`)) 10000.0)))
  (bind _outhit (`KismetSystemLibrary.LineTraceSingleForObjects` _returnvalue (+ _returnvalue (* (* (`self.GetActorUpVector`) (-1.0 -1.0 -1.0)) (15000.0 15000.0 15000.0))) (`|MakeArray` "ObjectTypeQuery1" :!type "EObjectTypeQuery Enum")))
  (`|SpawnActorFromClass` "/Game/Blueprints/BP_Enemy/BP_Enemy2.BP_Enemy2_C" (`KismetMathLibrary.MakeTransform` (`.ImpactPoint` (`GameplayStatics.BreakHitResult` _outhit))) "Undefined" "MultiplyWithRoot" null null))

(fn `UserConstructionScript`)