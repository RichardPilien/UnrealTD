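; Turret actor that sweeps for pawns tagged TurretTarget and fires projectiles at them in bursts.
; Tick runs a searching/attacking state machine, with searching swinging the Spine bone back and forth between yaw limits.
; PawnSensing sightings turn the bone toward the target, switch to attacking and restart a timer that resumes searching when sightings stop.
; Attacking launches BP_Projectile from the Arrow via physics velocity, gated by delays between shots and bursts.
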(event `self.ReceiveTick`
  (params (DeltaSeconds :type "Float (single-precision)"))
  ;[1 1 1] Calling State every frame
  (switch `/Game/Blueprints/BP_Units/Turret_State` (`self.TurretState`)
    (:`NewEnumerator0`
      (`self.SearchingTurret`))
    (:`NewEnumerator1`
      (`self.AttackingTurret`))))

(event `SearchingTurret`
  (bind _returnvalue (* (`GameplayStatics.GetWorldDeltaSeconds`) 50.0))
  ;[1 1 1] SearchingTurret moving Left and right
  (bind _returnvalue_2 (`PoseableMeshComponent.GetBoneRotationByName` (`self.Turret`) "Spine" "ComponentSpace"))
  (bind _yaw (.yaw _returnvalue_2))
  (set `self.ShouldTurretRotateRight` (or (and (< _yaw 70.0) (`self.ShouldTurretRotateRight`)) (and (< _yaw -70.0) (not (`self.ShouldTurretRotateRight`)))))
  (bind _yaw_2 (.yaw _returnvalue_2))
  (`PoseableMeshComponent.SetBoneRotationByName` (`self.Turret`) "Spine" (`KismetMathLibrary.MakeRotator` (.roll _returnvalue_2) (.pitch _returnvalue_2) (`KismetMathLibrary.SelectFloat` (+ _yaw_2 _returnvalue) (- _yaw_2 _returnvalue) (`self.ShouldTurretRotateRight`))) "ComponentSpace"))

(event `self.PawnSensing.OnSeePawn`
  (params (Pawn :type "Pawn Object Reference"))
  (bind _turret (`self.Turret`))
  (bind (_returnvalue_roll _returnvalue_pitch _returnvalue_yaw) (`KismetMathLibrary.BreakRotator` (`KismetMathLibrary.FindLookAtRotation` (`self.K2_GetActorLocation`) (`self.TargetLocation`))))
  ;[1 1 1] Rotation if looking at the target
  (if (`self.ActorHasTag` Pawn "TurretTarget")
    (set `self.TargetLocation` (`self.K2_GetActorLocation` Pawn))
    (set `self.TurretState` "NewEnumerator1")
    (bind _returnvalue (`PoseableMeshComponent.GetBoneRotationByName` _turret "Spine" "WorldSpace"))
    (`PoseableMeshComponent.SetBoneRotationByName` _turret "Spine" (`KismetMathLibrary.MakeRotator` (.roll _returnvalue) (.pitch _returnvalue) (- _returnvalue_yaw 90.0)) "WorldSpace")
    (`KismetSystemLibrary.K2_ClearAndInvalidateTimerHandle` (`self.ResetState`))
    (bind _returnvalue_2 (`KismetSystemLibrary.K2_SetTimerDelegate` (delegate `TurretReset`) 1.0))
    (set `self.ResetState` _returnvalue_2)))

(event `TurretReset`
  ;[1 1 1] Rotation if looking at the target
  (set `self.TurretState` "NewEnumerator0"))

(event `AttackingTurret`
  (bind _returnvalue (`SceneComponent.K2_GetComponentLocation` (`self.Arrow`)))
  (bind _returnvalue_2 (`KismetMathLibrary.GetDirectionUnitVector` _returnvalue (`self.TargetLocation`)))
  ;[1 1 1] Comment
  (if (not (`self.isAttacking?`))
    (set `self.isAttacking?` true)
    (bind _returnvalue_3 (`|SpawnActorFromClass` "/Game/Blueprints/BP_Units/BP_Projectile.BP_Projectile_C" (`KismetMathLibrary.MakeTransform` (+ _returnvalue (* _returnvalue_2 60.0))) "Undefined" "MultiplyWithRoot" null null))
    (`PrimitiveComponent.SetPhysicsLinearVelocity` (`/Game/Blueprints/BP_Units/BP_Projectile.Sphere` _returnvalue_3) (* _returnvalue_2 1000.0) false "None")
    (`KismetSystemLibrary.Delay` (`self.DelayAttack`))
    (bind _result (`/Engine/EditorBlueprintResources/StandardMacros.IncrementInt` (`self.NumberofAttack`))
      (:`  `
        (if (>= _result (`self.AttackFrequency`))
          (set `self.NumberofAttack` 0)
          (`KismetSystemLibrary.Delay` (`self.DelayBetweenMultilpleAttack`)))
        (set `self.isAttacking?` false)))))

(fn `UserConstructionScript`)